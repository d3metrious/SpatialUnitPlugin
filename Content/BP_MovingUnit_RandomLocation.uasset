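; Test-style moving unit that endlessly wanders to random navigable points around the player pawn, using SpatialMovement and SpatialEntity components.
; From BeginPlay it requests a debug move, retrying after a short delay on failure, and switches VARuntime between run and idle animations.
; On arrival it pauses, then picks a new point; an invalid avoidance event also triggers a new pick, with both events printing messages.
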(event `self.ReceiveBeginPlay`
  (`parent.ReceiveBeginPlay`)
  (`self.MoveToRandomLocation`))

(event `MoveToRandomLocation`
  (bind (_randomlocation _returnvalue) (`NavigationSystemV1.K2_GetRandomLocationInNavigableRadius` (`self.K2_GetActorLocation` (`GameplayStatics.GetPlayerPawn` 0)) 500.0 null null))
  (if _returnvalue
    (bind _returnvalue_2 (`SpatialMovementComponent.MoveTo` (`self.SpatialMovement`) _randomlocation null true true true))
    (if _returnvalue_2
      (`VARuntimeComponent.PlayAnimationByName` (`self.VARuntime`) "MF_Run_Fwd")
      (else
        (`KismetSystemLibrary.Delay` 0.2 :!label _label)
        (`self.MoveToRandomLocation`)))
    (else
      (goto _label))))

(event `self.SpatialMovement.OnTargetReached`
  (params (TargetActor :type "Actor Object Reference") (HitLocation :type "Vector Structure"))
  (`VARuntimeComponent.PlayAnimationByName` (`self.VARuntime`) "MF_Idle")
  (`KismetSystemLibrary.Delay` 1.0)
  (`self.MoveToRandomLocation`)
  (`KismetSystemLibrary.PrintString` "Target Reached"))

(event `self.SpatialEntity.OnAvoidance`
  (params (Velocity :type "Vector Structure (by ref)") (TargetLocation :type "Vector Structure (by ref)")))

(event `self.SpatialEntity.OnAvoidanceInvalid`
  (params (Velocity :type "Vector Structure (by ref)") (TargetLocation :type "Vector Structure (by ref)"))
  (`KismetSystemLibrary.PrintString` "OnAvoidance Invalid")
  (`self.MoveToRandomLocation`))

(fn `UserConstructionScript`
  (`parent.UserConstructionScript`))